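; BP_PPDGameMode is a game mode that sets up a cell map and shows a planned path on it.
; On BeginPlay it initializes the map, spawns a BP_PathPlanner and runs its path planning with itself as input.
; If planning succeeds, each entry of the returned path is looked up in MapInfo and the matching cell's type is set to Path.
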(event `self.ReceiveBeginPlay`
  (`self.InitMap`)
  (bind _returnvalue (`|SpawnActorFromClass` "/Game/Actors/BP_PathPlanner.BP_PathPlanner_C" (`KismetMathLibrary.MakeTransform` (0.0 0.0 0.0)) "Undefined" "MultiplyWithRoot" null null))
  (`/Engine/EditorBlueprintResources/StandardMacros.IsValid` _returnvalue
    (:`Is Valid`
      (set `self.PathPlannerRef` _returnvalue)
      (bind (_outpath _returnvalue_2) (`PPDPathPlanningActor.BPPathPlanning` (`self.PathPlannerRef`) self))
      (if _returnvalue_2
        (for _array_element _outpath
          (bind (_value _returnvalue_3) (`BlueprintMapLibrary.Map_Find` (`self.MapInfo`) _array_element))
          (if _returnvalue_3
            (`PPDCellBase.SetCellType` _value "ECT_Path")))))))

(fn `UserConstructionScript`)